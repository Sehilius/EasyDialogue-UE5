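; BP_EasyDialogueBox is a dialogue box in the DialogueGraph plugin functionality, holding styled dialogue text and optional player answers.
; GetMacroText joins the DialogueText segments into one string, wrapping each in rich-text style tags named from its Style enum.
; RequiresPlayerAnswer reports whether the box waits on a player choice, based solely on PlayerAnswers being non-empty.
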(fn RequiresPlayerAnswer
  (return (Utilities|Array|IsNotEmpty (Variables|Answers|GetPlayerAnswers))))

(fn GetMacroText
  (for _array_element (Variables|Basic|GetDialogueText)
    (LocalVariables|SetFinalTextLocal (Utilities|String|Append (LocalVariables|GetFinalTextLocal) (Utilities|String|Append (Utilities|String|Append "<" (Utilities|String|EnumtoString (.Style (Utilities|Struct|BreakF_EasyDialogueTextStyle _array_element))) ">") (.Text (Utilities|Struct|BreakF_EasyDialogueTextStyle _array_element)) "</>"))))
  (return (LocalVariables|GetFinalTextLocal)))
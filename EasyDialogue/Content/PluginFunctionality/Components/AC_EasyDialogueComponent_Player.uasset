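; Player-side dialogue component that lets the player talk to NPCs and drive the dialogue box.
; It creates the dialogue widget on BeginPlay, and interacting starts dialogue with the first overlapping actor that has an NPC dialogue component.
; Movement is disabled until the interaction finishes, while received dialogue data is passed to the widget.
; Proceed, fast-forward and answer navigation inputs are forwarded to the widget, gated by dialogue or answering state where needed.
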(event Custom|OnInteractionStarted
  (params (InteractableObject :type AC%20Easy%20Dialogue%20Component%20NPC%20Object%20Reference))
  ;[1 1 1] start interaction and freeze the player character
  (Default|OnInteractionStarted InteractableObject self)
  (Default|CallDisableMovement)
  (Variables|Default|SetCurrentlyInDialogue true))

(event Custom|OnInteractionFinished
  ;[1 1 1] reenable movement after interaction is finished
  (Default|CallEnableMovement)
  (Variables|Default|SetCurrentlyInDialogue false))

(event Custom|DialogueDataReceived
  (params (DialogueData :type Generic%20Graph%20Object%20Reference) (NPCDialogueComponent :type AC%20Easy%20Dialogue%20Component%20NPC%20Object%20Reference))
  ;[1 1 1] start the dialogue when data is received
  ;;[1 1 1] start displaying dialogue
  (Default|OnDialogueStarted (Variables|Default|GetDialogueWidget) DialogueData NPCDialogueComponent))

(event Custom|OnAnswerGiven
  ;[1 1 1] answering
  (Variables|Default|SetCurrentlyAnswering false))

(event Custom|OnAskedForAnswer
  ;[1 1 1] answering
  (Variables|Default|SetCurrentlyAnswering true))

(event Custom|OnToggleFastForward
  ;[1 1 1] fast forward the dialogue
  (if (Variables|/EasyDialogue/PluginFunctionality/BP_EasyDialogueTextAnimator.BP_EasyDialogueTextAnimator_C|GetIsFastForwardEnabled (Variables|/EasyDialogue/UserAssets/Widgets/WBP_EasyDialogueBox.WBP_EasyDialogueBox_C|GetTextAnimator (Variables|Default|GetDialogueWidget)))
    (Default|OnDisableFastForward (Variables|Default|GetDialogueWidget))
    (else
      (Default|OnEnableFastForward (Variables|Default|GetDialogueWidget)))))

(event Custom|OnTryToInteract
  (params (InteractionCollider :type Capsule%20Component%20Object%20Reference))
  ;[1 1 1] allow interaction only when currently not interacting
  (if (Variables|Default|GetCurrentlyInDialogue)
    (CallFunction|OnReceivedProceedInput)
    (else
      ;[1 1 1] start intreaction with the first interactable object found in overlaps
      (bind _array_element (Utilities|Array|ForEachLoopwithBreak (Collision|GetOverlappingActors InteractionCollider 0 :!class /Script/Engine.PrimitiveComponent) :!label _label)
        (:LoopBody
          (Utilities|IsValid (Actor|GetComponentbyClass _array_element "/EasyDialogue/PluginFunctionality/Components/AC_EasyDialogueComponent_NPC.AC_EasyDialogueComponent_NPC_C")
            (:Is%20Valid
              (CallFunction|OnInteractionStarted (Actor|GetComponentbyClass _array_element "/EasyDialogue/PluginFunctionality/Components/AC_EasyDialogueComponent_NPC.AC_EasyDialogueComponent_NPC_C"))
              (goto _label Break))))))))

(event Custom|OnAnswersMoveUp
  ;[1 1 1] answer selection
  (if (Variables|Default|GetCurrentlyAnswering)
    (Default|OnAnswerInputUp (Variables|Default|GetDialogueWidget))))

(event Custom|OnAnswersMoveDown
  ;[1 1 1] answer selection
  (if (Variables|Default|GetCurrentlyAnswering)
    (Default|OnAnswerInputDown (Variables|Default|GetDialogueWidget))))

(event Custom|OnReceivedProceedInput
  ;[1 1 1] can only proceed if currently in dialogue
  (if (Variables|Default|GetCurrentlyInDialogue)
    (Default|OnProceedInputReceived (Variables|Default|GetDialogueWidget))))

(event EventBeginPlay
  ;[1 1 1] create the dialogue widget specified in the settings
  (bind _returnvalue (UserInterface|CreateWidget "/EasyDialogue/UserAssets/Widgets/WBP_EasyDialogueBox.WBP_EasyDialogueBox_C"))
  (bind _output_get (Variables|Default|SetDialogueWidget _returnvalue))
  (UserInterface|Viewport|AddtoViewport _output_get 0)
  (Variables|/EasyDialogue/UserAssets/Widgets/WBP_EasyDialogueBox.WBP_EasyDialogueBox_C|SetPlayerCharacter (Variables|Default|GetDialogueWidget) self))

(event EventTick
  (params (DeltaSeconds :type Float%20%28single-precision%29)))
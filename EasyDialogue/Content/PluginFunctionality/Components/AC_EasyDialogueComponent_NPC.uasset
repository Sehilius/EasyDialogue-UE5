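; NPC-side dialogue component that hands the NPC's current dialogue to the player's dialogue component when an interaction starts.
; It passes CurrentDialogue and a self reference through DialogueDataReceived, while interaction finish does nothing.
; BindDialogueBoxEvent finds a dialogue box node by name and replaces any existing bindings on its fire event with the supplied one.
; A helper returns a random dialogue start sound.
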(event Custom|OnInteractionStarted
  (params (PlayerDialogueComponent :type AC%20Easy%20Dialogue%20Component%20Player%20Object%20Reference))
  ;[1 1 1] send the current dialogue data
  (Default|DialogueDataReceived PlayerDialogueComponent (Variables|Default|GetCurrentDialogue) self))

(event Custom|OnInteractionFinished)

(event EventBeginPlay)

(event EventTick
  (params (DeltaSeconds :type Float%20%28single-precision%29)))

(fn GetRandomDialogueStartSound
  (return (.OutItem (Utilities|Array|Random (Variables|Default|GetDialogueStartSounds)))))

(fn BindDialogueBoxEvent
  (params (DialogueBoxName :type Name%20%28by%20ref%29 :default "None"))
  (bind _array_element (Utilities|Array|ForEachLoopwithBreak (Variables|/Script/GenericGraphRuntime.GenericGraph|GetAllNodes (Variables|Default|GetCurrentDialogue)) :!label _label)
    (:LoopBody
      ;[1 1 1] search nodes for name
      (if (== (Variables|/EasyDialogue/PluginFunctionality/DialogueGraph/BP_EasyDialogueBox.BP_EasyDialogueBox_C|GetDialogueBoxName (.AsDialogue%20Box (Utilities|Casting|CastToBP_EasyDialogueBox _array_element))) DialogueBoxName)
        (LocalVariables|SetFoundNode (.AsDialogue%20Box (Utilities|Casting|CastToBP_EasyDialogueBox _array_element)))
        (goto _label Break)))
    (:Completed
      ;[1 1 1] only bind if node was found
      (Utilities|IsValid (LocalVariables|GetFoundNode)
        (:Is%20Valid
          ;[1 1 1] bind the event
          (EventDispatchers|UnbindallEventsfromOnFireDialogueEvent (LocalVariables|GetFoundNode))
          (EventDispatchers|BindEventtoOnFireDialogueEvent (LocalVariables|GetFoundNode) (Variables|Default|GetDialogueBoxEvent)))))))
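; BP_QuestBall is a collectible quest ball for the demo world that stays hidden without collision until its quest starts.
; OnStartQuest reveals the ball and enables query and physics collision on its Sphere.
; When the Easy Dialogue player character overlaps it, it calls OnBallCollected on both that character and the Vitta reference, then destroys itself.
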(event Custom|OnStartQuest
  ;[1 1 1] "spawn" the ball when the quests starts
  (Collision|SetCollisionEnabled (Variables|Default|GetSphere) "QueryAndPhysics")
  (Rendering|SetActorHiddenInGame false))

(event EventBeginPlay
  ;[1 1 1] hide the ball on game start
  (Collision|SetCollisionEnabled (Variables|Default|GetSphere) "NoCollision")
  (Rendering|SetActorHiddenInGame true))

(event Collision|EventActorBeginOverlap
  (params (OtherActor :type Actor%20Object%20Reference))
  (bind _asbp_dialogue_player_character (Utilities|Casting|CastToBP_EasyDialoguePlayerCharacter OtherActor))
  (Default|OnBallCollected _asbp_dialogue_player_character)
  (Default|OnBallCollected (Variables|Default|GetVitta))
  (Actor|DestroyActor))

(event EventTick
  (params (DeltaSeconds :type Float%20%28single-precision%29)))

(fn ConstructionScript)
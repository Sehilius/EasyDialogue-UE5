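; NPC Blueprint for Vitta, who gives a ball quest through her dialogue component.
; On BeginPlay it registers a delegate for the "BallQuestStart" dialogue box event.
; StartBallQuest notifies the QuestBall that the quest has begun.
; OnBallCollected switches her current dialogue to her second dialogue, Dialogue_Vitta_2.
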(event Custom|StartBallQuest
  ;[1 1 1] start the ball quest
  (Default|OnStartQuest (Variables|Default|GetQuestBall)))

(event Custom|OnBallCollected
  ;[1 1 1] when the ball is collected, change vitta's dialogue
  (Variables|/EasyDialogue/PluginFunctionality/Components/AC_EasyDialogueComponent_NPC.AC_EasyDialogueComponent_NPC_C|SetCurrentDialogue (Variables|Default|GetAC_DialogueComponent) "/EasyDialogue/DemoWorld/Dialogues/Dialogue_Vitta_2.Dialogue_Vitta_2"))

(event EventBeginPlay
  (|CallParentFunction)
  (Class|DialogueComponent|SetDialogueBoxEvent (Variables|Default|GetAC_DialogueComponent) (EventDispatchers|CreateEvent :!event Custom|StartBallQuest) "BallQuestStart"))

(event Collision|EventActorBeginOverlap
  (params (OtherActor :type Actor%20Object%20Reference))
  (|CallParentFunction OtherActor) ; This node is disabled and will not be called.\nDrag off pins to build functionality.
)

(event EventTick
  (params (DeltaSeconds :type Float%20%28single-precision%29))
  (|CallParentFunction DeltaSeconds) ; This node is disabled and will not be called.\nDrag off pins to build functionality.
)

(fn ConstructionScript
  (|CallParentFunction))
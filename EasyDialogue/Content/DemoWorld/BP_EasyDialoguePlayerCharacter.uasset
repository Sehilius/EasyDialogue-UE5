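; Demo player character for the Easy Dialogue system, handling interaction, dialogue controls and a flag for collecting the kid's ball.
; On BeginPlay it adds the dialogue input mapping context and creates the player dialogue component at runtime.
; Enhanced Input actions forward interact, fast-forward and answer selection to that component.
; The component's movement events are bound back to the character to disable and restore walking.
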(event Custom|OnBallCollected
  ;[1 1 1] when player collects the kid's ball
  (Variables|Default|SetPossessesBall true))

(event Custom|DisableMovement
  ;[1 1 1] movement management for dialogue
  (Pawn|Components|CharacterMovement|DisableMovement (Variables|Character|GetCharacterMovement)))

(event Custom|EnableMovement
  ;[1 1 1] movement management for dialogue
  (Pawn|Components|CharacterMovement|SetMovementMode (Variables|Character|GetCharacterMovement) "MOVE_Walking" 0))

(event Input|EnhancedActionEvents|EnhancedInputActionIA_Interact
  (params (ActionValue :type Boolean) (ElapsedSeconds :type Float%20%28double-precision%29) (TriggeredSeconds :type Float%20%28double-precision%29) (InputAction :type Input%20Action%20Object%20Reference :default "/EasyDialogue/DemoWorld/Controls/Actions/IA_Interact.IA_Interact"))
  ;[1 1 1] interact
  (:Started
    (Default|OnTrytoInteract (Variables|Default|GetDialogueComponent) (Variables|Default|GetInteractionCollider))))

(event Input|EnhancedActionEvents|EnhancedInputActionIA_ToggleFastForward
  (params (ActionValue :type Boolean) (ElapsedSeconds :type Float%20%28double-precision%29) (TriggeredSeconds :type Float%20%28double-precision%29) (InputAction :type Input%20Action%20Object%20Reference :default "/EasyDialogue/DemoWorld/Controls/Actions/IA_ToggleFastForward.IA_ToggleFastForward"))
  (bind _dialoguecomponent (Variables|Default|GetDialogueComponent))
  ;[1 1 1] fast forward
  (:Started
    (if (Variables|/EasyDialogue/PluginFunctionality/Components/AC_EasyDialogueComponent_Player.AC_EasyDialogueComponent_Player_C|GetCurrentlyInDialogue _dialoguecomponent)
      (Default|OnToggleFastForward _dialoguecomponent))))

(event Input|EnhancedActionEvents|EnhancedInputActionIA_AnswerMoveUp
  (params (ActionValue :type Boolean) (ElapsedSeconds :type Float%20%28double-precision%29) (TriggeredSeconds :type Float%20%28double-precision%29) (InputAction :type Input%20Action%20Object%20Reference :default "/EasyDialogue/DemoWorld/Controls/Actions/IA_AnswerMoveUp.IA_AnswerMoveUp"))
  ;[1 1 1] answer selection
  (:Started
    (Default|OnAnswersMoveUp (Variables|Default|GetDialogueComponent))))

(event Input|EnhancedActionEvents|EnhancedInputActionIA_AnswerMoveDown
  (params (ActionValue :type Boolean) (ElapsedSeconds :type Float%20%28double-precision%29) (TriggeredSeconds :type Float%20%28double-precision%29) (InputAction :type Input%20Action%20Object%20Reference :default "/EasyDialogue/DemoWorld/Controls/Actions/IA_AnswerMoveDown.IA_AnswerMoveDown"))
  ;[1 1 1] answer selection
  (:Started
    (Default|OnAnswersMoveDown (Variables|Default|GetDialogueComponent))))

(event EventBeginPlay
  (Utilities|FlowControl|Sequence
    (:then_0
      ;[1 1 1] set input mappings
      (bind _asplayer_controller (Utilities|Casting|CastToPlayerController (Pawn|GetController)))
      (Utilities|IsValid (PlayerController|LocalPlayerSubsystems|GetEnhancedInputLocalPlayerSubsystem _asplayer_controller)
        (:Is%20Valid
          (Input|AddMappingContext (PlayerController|LocalPlayerSubsystems|GetEnhancedInputLocalPlayerSubsystem _asplayer_controller) "/EasyDialogue/DemoWorld/Controls/IMC_EasyDialogueActionMappings.IMC_EasyDialogueActionMappings" 0 "(bIgnoreAllPressedKeysUntilRelease=True,bForceImmediately=False)"))))
    (:then_1
      (bind _returnvalue (Game|AddComponentbyClass "/EasyDialogue/PluginFunctionality/Components/AC_EasyDialogueComponent_Player.AC_EasyDialogueComponent_Player_C"))
      ;[1 1 1] bind mandatory events
      (bind _output_get (Variables|Default|SetDialogueComponent _returnvalue))
      (EventDispatchers|BindEventtoDisableMovement _output_get (EventDispatchers|CreateEvent :!event Custom|DisableMovement))
      (EventDispatchers|BindEventtoEnableMovement _returnvalue (EventDispatchers|CreateEvent :!event Custom|EnableMovement)))))

(event Collision|EventActorBeginOverlap
  (params (OtherActor :type Actor%20Object%20Reference)))

(fn ConstructionScript
  (|CallParentFunction))
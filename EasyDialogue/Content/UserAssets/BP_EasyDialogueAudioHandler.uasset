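; Audio handler actor for the EasyDialogue system that plays music, voice lines and UI sounds during dialogue.
; On BeginPlay it adds separate audio components for music and voice lines, then starts the level music.
; Events play or stop each channel, while short sounds fire as unstoppable 2D one-shots, including global cues read from dialogue settings.
; When dialogue finishes, it restores the level music unless that is already set.
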(event Custom|OnPlaySound
  (params (Sound :type Sound%20Wave%20Object%20Reference))
  ;[1 1 1] short sounds that cannot and do not need to be stopped
  (Utilities|IsValid Sound
    (:Is%20Valid
      (Audio|PlaySound2D Sound 1.0 1.0 0.0 0 0))))

(event Custom|OnPlayVoiceLine
  (params (Music :type Sound%20Wave%20Object%20Reference))
  ;[1 1 1] voice lines
  (Audio|Components|Audio|SetSound (Variables|Default|GetVoiceLineAudioComponent) Music)
  (Audio|Components|Audio|Play (Variables|Default|GetVoiceLineAudioComponent) 0.0))

(event Custom|OnPlayFastForwardEnabledSound
  (bind _dialoguesettings (CallFunction|GetDialogueSettings))
  (bind _fastforwardenabledsound (Variables|/Script/EasyDialogue.DialogueSettings|GetFastForwardEnabledSound _dialoguesettings))
  ;[1 1 1] game wide sounds
  (Utilities|IsValid _fastforwardenabledsound
    (:Is%20Valid
      (CallFunction|OnPlaySound _fastforwardenabledsound))))

(event Custom|FastForwardDisabledSound
  (bind _dialoguesettings (CallFunction|GetDialogueSettings))
  (bind _fastforwarddisabledsound (Variables|/Script/EasyDialogue.DialogueSettings|GetFastForwardDisabledSound _dialoguesettings))
  ;[1 1 1] game wide sounds
  (Utilities|IsValid _fastforwarddisabledsound
    (:Is%20Valid
      (CallFunction|OnPlaySound _fastforwarddisabledsound))))

(event Custom|OnPlayMusic
  (params (Music :type Sound%20Wave%20Object%20Reference))
  ;[1 1 1] music
  (Utilities|IsValid Music
    (:Is%20Valid
      (Audio|Components|Audio|SetSound (Variables|Default|GetMusicAudioComponent) Music)
      (Audio|Components|Audio|Play (Variables|Default|GetMusicAudioComponent) 0.0))))

(event Custom|OnStopVoiceLine
  ;[1 1 1] voice lines
  (Audio|Components|Audio|Stop (Variables|Default|GetVoiceLineAudioComponent)))

(event Custom|OnStopMusic
  ;[1 1 1] music
  (Audio|Components|Audio|Stop (Variables|Default|GetMusicAudioComponent)))

(event Custom|OnDialogueFinished
  ;[1 1 1] play the specified music of the level
  ;;[1 1 1] is the level music already playing?
  (if (!= (Variables|Default|GetLevelMusic) (Variables|/Script/Engine.AudioComponent|GetSound (Variables|Default|GetMusicAudioComponent)))
    (CallFunction|OnPlayLevelMusic)))

(event Custom|OnPlayHoverAnswerSound
  (bind _dialoguesettings (CallFunction|GetDialogueSettings))
  (bind _hoveranswersound (Variables|/Script/EasyDialogue.DialogueSettings|GetHoverAnswerSound _dialoguesettings))
  ;[1 1 1] game wide sounds
  (Utilities|IsValid _hoveranswersound
    (:Is%20Valid
      (CallFunction|OnPlaySound _hoveranswersound))))

(event Custom|OnPlayProceedSound
  (bind _dialoguesettings (CallFunction|GetDialogueSettings))
  (bind _proceedsound (Variables|/Script/EasyDialogue.DialogueSettings|GetProceedSound _dialoguesettings))
  ;[1 1 1] game wide sounds
  (Utilities|IsValid _proceedsound
    (:Is%20Valid
      (CallFunction|OnPlaySound _proceedsound))))

(event Custom|OnPlayLevelMusic
  (CallFunction|OnPlayMusic (Variables|Default|GetLevelMusic)))

(event Custom|OnPlayGiveAnswerSound
  (bind _dialoguesettings (CallFunction|GetDialogueSettings))
  (bind _giveanswersound (Variables|/Script/EasyDialogue.DialogueSettings|GetGiveAnswerSound _dialoguesettings))
  ;[1 1 1] game wide sounds
  (Utilities|IsValid _giveanswersound
    (:Is%20Valid
      (CallFunction|OnPlaySound _giveanswersound))))

(event EventBeginPlay
  ;[1 1 1] audio component for music
  (bind _returnvalue (AddComponent|AddAudioComponent false))
  (Variables|Default|SetMusicAudioComponent _returnvalue)
  ;[1 1 1] audio component for voice lines
  (bind _returnvalue_2 (AddComponent|AddAudioComponent false))
  (Variables|Default|SetVoiceLineAudioComponent _returnvalue_2)
  ;[1 1 1] play the level's music
  (CallFunction|OnPlayLevelMusic))

(event Collision|EventActorBeginOverlap
  (params (OtherActor :type Actor%20Object%20Reference)))

(event EventTick
  (params (DeltaSeconds :type Float%20%28single-precision%29)))

(fn ConstructionScript)